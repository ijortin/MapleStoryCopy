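; Base player character for a networked 2D side-scroller, handling left/right movement and a ground-only jump.
; The move axis drives movement along the control rotation's forward vector and derives an idle, run, jump or fall state from input and velocity.
; That state passes through an SRV event into MovementState, whose OnRep swaps PlayerInfo flipbooks and rotates the sprite to face the run direction.
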(event Custom|SetMovementState
  (params (MovementState :type E_MovementState%20Enum :default "NewEnumerator0"))
  (CallFunction|SRVSetMovementState MovementState))

(event Custom|SRV_SetMovementState
  (params (MovementState :type E_MovementState%20Enum :default "NewEnumerator0"))
  (Variables|Default|SetMovementState MovementState))

(event EventBeginPlay)

(event Collision|EventActorBeginOverlap
  (params (OtherActor :type Actor%20Object%20Reference)))

(event EventTick
  (params (DeltaSeconds :type Float%20%28single-precision%29)))

(event Input|ActionEvents|InputActionJump
  (params (Key :type Key%20Structure :default "None"))
  ;[1 1 1] PlayerMovement (JUMP)
  (:Pressed
    (if (not (AI|Components|NavMovement|IsFalling (Variables|Character|GetCharacterMovement))) ; TODO: Add flashjumps to "True" branch.
      (Character|Jump))))

(event Input|AxisEvents|InputAxisMoveRight/Left
  (params (AxisValue :type Float%20%28single-precision%29))
  ;[1 1 1] PlayerMovement (RIGHT and LEFT)
  (Pawn|Input|AddMovementInput (Math|Vector|GetForwardVector (Pawn|GetControlRotation :!class /Script/Engine.Pawn)) AxisValue false)
  (if (AI|Components|NavMovement|IsFalling (Variables|Character|GetCharacterMovement))
    (if (> (.Z (Math|Vector|BreakVector (Transformation|GetVelocity))) 0.0)
      (CallFunction|SetMovementState "NewEnumerator3")
      (else
        (CallFunction|SetMovementState "NewEnumerator4")))
    (elif (== AxisValue 0.0)
      (CallFunction|SetMovementState "NewEnumerator0")
      (elif (> AxisValue 0.0)
        (CallFunction|SetMovementState "NewEnumerator1")
        (else
          (CallFunction|SetMovementState "NewEnumerator2"))))))

(fn ConstructionScript
  (|CallParentFunction))

(fn OnRepMovementState
  (bind _sprite (Variables|Default|GetSprite))
  (bind _playerinfo (Variables|Default|GetPlayerInfo))
  (bind (_idleanimation _walkanimation _jumpanimation _fallanimation) (Utilities|Struct|BreakST_PlayerInfo _playerinfo))
  (switch Utilities|FlowControl|Switch|SwitchonE_MovementState (Variables|Default|GetMovementState)
    (:NewEnumerator0
      (Sprite|SetFlipbook _sprite _idleanimation))
    (:NewEnumerator1
      (Transformation|SetRelativeRotation _sprite "0.000000,180.000000,0.000000" false false)
      (Sprite|SetFlipbook _sprite _walkanimation))
    (:NewEnumerator2
      (Transformation|SetRelativeRotation _sprite "0, 0, 0" false false)
      (Sprite|SetFlipbook _sprite _walkanimation))
    (:NewEnumerator3
      (Sprite|SetFlipbook _sprite _jumpanimation))
    (:NewEnumerator4
      (Sprite|SetFlipbook _sprite _fallanimation))))